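; Hinged door Blueprint that toggles open and closed through OpenDoor, first consuming the player's key if it is locked.
; A FlipFlop alternates playing and reversing the DoorAction timeline, which lerps the Pivot's rotation.
; Short retriggerable-delay loops reissue Play or Reverse until the timeline finishes.
; A Player-tagged actor entering the Box stops the timeline, which an active loop then resumes.
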(event OnComponentBeginOverlap(Box)
  (params (OverlappedComponent :type Primitive%20Component%20Object%20Reference) (OtherActor :type Actor%20Object%20Reference) (OtherComp :type Primitive%20Component%20Object%20Reference) (OtherBodyIndex :type Integer) (bFromSweep :type Boolean) (SweepResult :type Hit%20Result%20Structure%20%28by%20ref%29))
  (if (Actor|ActorHasTag OtherActor "Player")
    (Development|PrintString "gangin")
    (bind _lerpvalue (Timeline|DoorAction Stop)
      (:Update
        (Transformation|SetRelativeRotation (Variables|Default|GetPivot) (Math|Rotator|Lerp(Rotator) "0, 0, 0" "0,100.000000, 0" _lerpvalue) false false))
      (:Finished
        (Variables|Default|SetContinue false)))))

(event Custom|OpenDoor
  (bind _as_bp_player_character (Variables|Default|GetAs%20BP%20Player%20Character))
  (if (Variables|Default|GetKeyNeeded)
    (if (Variables|/Game/Blueprints/PlayerCPP/BP_PlayerCharacter.BP_PlayerCharacter_C|GethasKey? _as_bp_player_character)
      (Variables|/Game/Blueprints/PlayerCPP/BP_PlayerCharacter.BP_PlayerCharacter_C|SethasKey? _as_bp_player_character false)
      (Variables|Default|SetKeyNeeded false)
      (Variables|Default|SetContinue true :!label _label)
      (bind _isa (Utilities|FlowControl|FlipFlop)
        (:A
          (if (and (Variables|Default|GetContinue) _isa) :!label _label_2
            (Utilities|FlowControl|RetriggerableDelay 0.01)
            (Utilities|FlowControl|Sequence
              (:then_0
                (goto _label_2))
              (:then_1
                (bind _lerpvalue (Timeline|DoorAction Play)
                  (:Update
                    (Transformation|SetRelativeRotation (Variables|Default|GetPivot) (Math|Rotator|Lerp(Rotator) "0, 0, 0" "0,100.000000, 0" _lerpvalue) false false))
                  (:Finished
                    (Variables|Default|SetContinue false)))))))
        (:B
          (if (and (Variables|Default|GetContinue) (not _isa)) :!label _label_3
            (Utilities|FlowControl|RetriggerableDelay 0.01)
            (Utilities|FlowControl|Sequence
              (:then_0
                (goto _label_3))
              (:then_1
                (Timeline|DoorAction Reverse)))))))
    (else
      (goto _label))))

(event EventBeginPlay
  (bind _asbp_player_character (Utilities|Casting|CastToBP_PlayerCharacter (Game|GetPlayerCharacter 0)))
  (Variables|Default|SetAs%20BP%20Player%20Character _asbp_player_character))

(fn ConstructionScript)