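; BP_Boundary is a boundary volume that returns objects and the player when they overlap its collision.
; On begin overlap, a BP_MovableObject has its Respawn function called.
; A FirstPersonCharacter instead has its capsule moved to the world location of the referenced PlayerRespawnPoint, if one is valid, without sweep or teleport physics.
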(event OnComponentBeginOverlap(Collision)
  (params (OverlappedComponent :type Primitive%20Component%20Object%20Reference) (OtherActor :type Actor%20Object%20Reference) (OtherComp :type Primitive%20Component%20Object%20Reference) (OtherBodyIndex :type Integer) (bFromSweep :type Boolean) (SweepResult :type Hit%20Result%20Structure%20%28by%20ref%29))
  (bind _playerrespawnpoint (Variables|Default|GetPlayerRespawnPoint))
  (Utilities|FlowControl|Sequence
    (:then_0
      (bind _asbp_movable_object (Utilities|Casting|CastToBP_MovableObject OtherActor))
      (Utilities|IsValid _asbp_movable_object
        (:Is%20Valid
          (Default|Respawn _asbp_movable_object))))
    (:then_1
      (bind _asfirst_person_character (Utilities|Casting|CastToFirstPersonCharacter OtherActor))
      (Utilities|IsValid _asfirst_person_character
        (:Is%20Valid
          (Utilities|IsValid _playerrespawnpoint
            (:Is%20Valid
              (Transformation|SetWorldLocation (Variables|/Script/Engine.Character|GetCapsuleComponent _asfirst_person_character) (Transformation|GetWorldLocation (Variables|/Game/Blueprints/BP_PlayerRespawnPoint.BP_PlayerRespawnPoint_C|GetDefaultSceneRoot _playerrespawnpoint)) false false))))))))

(fn ConstructionScript)