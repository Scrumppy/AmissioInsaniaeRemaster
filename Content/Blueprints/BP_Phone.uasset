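; Phone actor that plays sound on proximity and pickup, and ends the game when flagged as the final phone.
; Box overlap starts the cue audio once if PlaySound is set, while Sphere overlap plays the pickup sound once.
; With both PlaySound and FinalPhone set, pickup also disables player movement, switches to UI-only input, then shows a fade-out widget and loads the main menu after timed delays.
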(event OnComponentBeginOverlap(Box)
  (params (OverlappedComponent :type Primitive%20Component%20Object%20Reference) (OtherActor :type Actor%20Object%20Reference) (OtherComp :type Primitive%20Component%20Object%20Reference) (OtherBodyIndex :type Integer) (bFromSweep :type Boolean) (SweepResult :type Hit%20Result%20Structure%20%28by%20ref%29))
  (if (Variables|Default|GetPlaySound?)
    (Utilities|FlowControl|DoOnce false
      (:Completed
        (Audio|Components|Audio|Play (Variables|Default|GetBeginCue) 0.0)))))

(event OnComponentBeginOverlap(Sphere)
  (params (OverlappedComponent :type Primitive%20Component%20Object%20Reference) (OtherActor :type Actor%20Object%20Reference) (OtherComp :type Primitive%20Component%20Object%20Reference) (OtherBodyIndex :type Integer) (bFromSweep :type Boolean) (SweepResult :type Hit%20Result%20Structure%20%28by%20ref%29))
  (if (and (Variables|Default|GetPlaySound?) (Variables|Default|GetFinal%20Phone?))
    (Utilities|FlowControl|DoOnce false
      (:Completed
        (bind _asbp_player_character (Utilities|Casting|CastToBP_PlayerCharacter (Game|GetPlayerCharacter 0)))
        (Audio|PlaySoundatLocation (Variables|Default|GetPickupSound) (Transformation|GetActorLocation) "0, 0, 0" 1.0 1.0 0.0 0 0 0 0)
        (Utilities|FlowControl|Sequence
          (:then_0
            (Utilities|FlowControl|Delay 12.0)
            (bind _returnvalue (UserInterface|CreateWidget "/Game/UI/EndFade/WBP_FadeOut.WBP_FadeOut_C"))
            (UserInterface|Viewport|AddtoViewport _returnvalue 0)
            (Utilities|FlowControl|Delay 6.0)
            (Game|OpenLevel(byName) "MainMenuLevel"))
          (:then_1
            (Pawn|Components|CharacterMovement|DisableMovement (Variables|/Script/Engine.Character|GetCharacterMovement _asbp_player_character))
            (Utilities|FlowControl|Delay 4.0)
            (Input|SetInputModeUIOnly (Game|GetPlayerController 0) _returnvalue "DoNotLock" false)))))
    (else
      (Utilities|FlowControl|DoOnce false
        (:Completed
          (Utilities|Casting|CastToBP_PlayerCharacter (Game|GetPlayerCharacter 0))
          (Audio|PlaySoundatLocation (Variables|Default|GetPickupSound) (Transformation|GetActorLocation) "0, 0, 0" 1.0 1.0 0.0 0 0 0 0))))))

(fn ConstructionScript)