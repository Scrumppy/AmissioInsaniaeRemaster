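; BP_Radio is a radio actor that plays its BeginCue audio once, on the first overlap with its sphere.
; The cast tests player character 0 rather than the overlapping actor, so any overlapping actor can use up the DoOnce.
; BeginPlay holds a Delay that leads nowhere.
; A chain that stops the cue and plays a pickup sound at the actor's location is never run.
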(event OnComponentBeginOverlap(Sphere)
  (params (OverlappedComponent :type Primitive%20Component%20Object%20Reference) (OtherActor :type Actor%20Object%20Reference) (OtherComp :type Primitive%20Component%20Object%20Reference) (OtherBodyIndex :type Integer) (bFromSweep :type Boolean) (SweepResult :type Hit%20Result%20Structure%20%28by%20ref%29))
  (Utilities|FlowControl|DoOnce false
    (:Completed
      (Utilities|Casting|CastToBP_PlayerCharacter (Game|GetPlayerCharacter 0))
      (Audio|Components|Audio|Play (Variables|Default|GetBeginCue) 0.0))))

(event EventBeginPlay
  (Utilities|FlowControl|Delay 4e+01))

(fn ConstructionScript)