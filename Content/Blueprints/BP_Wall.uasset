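; BP_Wall is a wall actor whose Cube mesh can be switched on or off.
; On BeginPlay it reads the Active flag and calls either ActivateMesh or DisableMesh.
; These two custom events set visibility and collision together, so a disabled wall is both hidden and passable.
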(event Custom|DisableMesh
  (bind _cube (Variables|Default|GetCube))
  (Rendering|SetVisibility _cube false false)
  (Collision|SetCollisionEnabled _cube "NoCollision"))

(event Custom|ActivateMesh
  (bind _cube (Variables|Default|GetCube))
  (Rendering|SetVisibility _cube true false)
  (Collision|SetCollisionEnabled _cube "QueryAndPhysics"))

(event EventBeginPlay
  (if (Variables|Default|GetActive?)
    (CallFunction|ActivateMesh)
    (else
      (CallFunction|DisableMesh))))

(fn ConstructionScript)