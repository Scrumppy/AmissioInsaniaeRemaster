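; Trigger volume that switches a linked Wall and Door on or off when the player walks into it.
; The ActivateMesh flag decides whether both are activated or disabled.
; On overlap it also destroys an optional paired trigger, OtherTrigger.
; BeginPlay applies the same wall and door state immediately whenever a save game exists in the game instance's slot, without waiting for an overlap.
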(event OnComponentBeginOverlap(Box)
  (params (OverlappedComponent :type Primitive%20Component%20Object%20Reference) (OtherActor :type Actor%20Object%20Reference) (OtherComp :type Primitive%20Component%20Object%20Reference) (OtherBodyIndex :type Integer) (bFromSweep :type Boolean) (SweepResult :type Hit%20Result%20Structure%20%28by%20ref%29))
  (bind _wall (Variables|Default|GetWall))
  (bind _othertrigger (Variables|Default|GetOtherTrigger))
  (bind _activatemesh_ (Variables|Default|GetActivateMesh?))
  (bind _door (Variables|Default|GetDoor))
  (Utilities|Casting|CastToBP_PlayerCharacter OtherActor)
  (Utilities|FlowControl|Sequence
    (:then_0
      (if _activatemesh_
        (Variables|/Game/Blueprints/BP_Wall.BP_Wall_C|SetActive? _wall _activatemesh_)
        (Default|ActivateMesh _wall)
        (Variables|/Game/Blueprints/BP_Wall.BP_Wall_C|SetActive? _door _activatemesh_)
        (Default|ActivateMesh _door)
        (else
          (Variables|/Game/Blueprints/BP_Wall.BP_Wall_C|SetActive? _wall _activatemesh_)
          (Default|DisableMesh _wall)
          (Variables|/Game/Blueprints/BP_Wall.BP_Wall_C|SetActive? _door _activatemesh_)
          (Default|DisableMesh _door))))
    (:then_1
      (Utilities|IsValid _othertrigger
        (:Is%20Valid
          (Actor|DestroyActor _othertrigger))))))

(event EventBeginPlay
  (bind _wall (Variables|Default|GetWall))
  (bind _activatemesh_ (Variables|Default|GetActivateMesh?))
  (bind _door (Variables|Default|GetDoor))
  (bind _returnvalue (SaveGame|DoesSaveGameExist (Variables|/Game/AmissioGameInstance.AmissioGameInstance_C|GetSave%20Slot%20Name (.AsAmissio%20Game%20Instance (Utilities|Casting|CastToAmissioGameInstance (Game|GetGameInstance))))))
  (if _returnvalue
    (if _activatemesh_
      (Variables|/Game/Blueprints/BP_Wall.BP_Wall_C|SetActive? _wall _activatemesh_)
      (Default|ActivateMesh _wall)
      (Variables|/Game/Blueprints/BP_Wall.BP_Wall_C|SetActive? _door _activatemesh_)
      (Default|ActivateMesh _door)
      (else
        (Variables|/Game/Blueprints/BP_Wall.BP_Wall_C|SetActive? _wall _activatemesh_)
        (Default|DisableMesh _wall)
        (Variables|/Game/Blueprints/BP_Wall.BP_Wall_C|SetActive? _door _activatemesh_)
        (Default|DisableMesh _door)))))

(fn ConstructionScript)