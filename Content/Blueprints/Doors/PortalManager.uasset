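; Manager that links two Portal actors into a see-through pair and moves overlapping actors from one to the other.
; On BeginPlay it casts both portals and swaps their Entrance materials, so each shows the other's material.
; Every tick it places each portal's Capture at the player camera's transform mapped through the pair with a 180-degree yaw flip.
; Overlaps set the actor's location to the opposite portal's root, with no rotation change or re-entry guard.
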(event OnActorBeginOverlap(AsPortalTwo)
  (params (OverlappedActor :type Actor%20Object%20Reference) (OtherActor :type Actor%20Object%20Reference))
  (Transformation|SetActorLocation OtherActor (Transformation|GetWorldLocation (Variables|/Game/Blueprints/Doors/Portal.Portal_C|GetDefaultSceneRoot (Variables|Default|GetAs%20Portal%20One))) false false))

(event OnActorBeginOverlap(Portal1)
  (params (OverlappedActor :type Actor%20Object%20Reference) (OtherActor :type Actor%20Object%20Reference))
  (Development|PrintString "Hello")
  (Transformation|SetActorLocation OtherActor (Transformation|GetWorldLocation (Variables|/Game/Blueprints/Doors/Portal.Portal_C|GetDefaultSceneRoot (Variables|Default|GetAs%20Portal%20Two))) false false))

(event EventBeginPlay
  (bind _asportal (Utilities|Casting|CastToPortal (Variables|Default|GetPortal1)))
  (bind _output_get (Variables|Default|SetAs%20Portal%20One _asportal))
  (Variables|Default|SetPortalOneMaterial (Rendering|Material|GetMaterial (Variables|/Game/Blueprints/Doors/Portal.Portal_C|GetEntrance _output_get) 0))
  (bind _asportal_2 (Utilities|Casting|CastToPortal (Variables|Default|GetPortal2)))
  (bind _output_get_2 (Variables|Default|SetAs%20Portal%20Two _asportal_2))
  (Variables|Default|SetPortalTwoMaterial (Rendering|Material|GetMaterial (Variables|/Game/Blueprints/Doors/Portal.Portal_C|GetEntrance _output_get_2) 0))
  (Rendering|Material|SetMaterial (Variables|/Game/Blueprints/Doors/Portal.Portal_C|GetEntrance (Variables|Default|GetAs%20Portal%20One)) 0 (Variables|Default|GetPortalTwoMaterial))
  (Rendering|Material|SetMaterial (Variables|/Game/Blueprints/Doors/Portal.Portal_C|GetEntrance (Variables|Default|GetAs%20Portal%20Two)) 0 (Variables|Default|GetPortalOneMaterial)))

(event Collision|EventActorBeginOverlap
  (params (OtherActor :type Actor%20Object%20Reference)))

(event EventTick
  (params (DeltaSeconds :type Float%20%28single-precision%29))
  (CallFunction|UpdatePortal1)
  (CallFunction|UpdatePortal2))

(fn ConstructionScript)

(fn UpdatePortal1
  (bind _returnvalue (Game|GetPlayerCameraManager 0))
  (bind _as_portal_two (Variables|Default|GetAs%20Portal%20Two))
  (bind _as_portal_one (Variables|Default|GetAs%20Portal%20One))
  (bind _defaultsceneroot (Variables|/Game/Blueprints/Doors/Portal.Portal_C|GetDefaultSceneRoot _as_portal_one))
  (bind _defaultsceneroot_2 (Variables|/Game/Blueprints/Doors/Portal.Portal_C|GetDefaultSceneRoot _as_portal_two))
  (bind _transformcomponent (Variables|/Script/Engine.PlayerCameraManager|GetTransformComponent _returnvalue))
  (bind _returnvalue_2 (Transformation|GetWorldRotation _defaultsceneroot_2))
  (bind _returnvalue_3 (Transformation|GetWorldRotation _defaultsceneroot))
  (bind _returnvalue_4 (- (.yaw _returnvalue_2) 1.8e+02))
  (bind _returnvalue_5 (Math|Rotator|MakeRotator (.roll _returnvalue_2) (.pitch _returnvalue_2) _returnvalue_4))
  (bind _returnvalue_6 (Math|Rotator|Delta(Rotator) _returnvalue_5 _returnvalue_3))
  (Transformation|SetWorldLocationAndRotation (Variables|/Game/Blueprints/Doors/Portal.Portal_C|GetCapture (Variables|Default|GetAs%20Portal%20Two)) (+ (- (Transformation|GetWorldLocation _defaultsceneroot_2) (Math|Vector|RotateVector (Transformation|GetWorldLocation _defaultsceneroot) _returnvalue_6)) (Math|Vector|RotateVector (Transformation|GetWorldLocation _transformcomponent) _returnvalue_6)) (Math|Rotator|CombineRotators (Transformation|GetWorldRotation _transformcomponent) _returnvalue_6) false false))

(fn UpdatePortal2
  (bind _returnvalue (Game|GetPlayerCameraManager 0))
  (bind _as_portal_one (Variables|Default|GetAs%20Portal%20One))
  (bind _as_portal_two (Variables|Default|GetAs%20Portal%20Two))
  (bind _defaultsceneroot (Variables|/Game/Blueprints/Doors/Portal.Portal_C|GetDefaultSceneRoot _as_portal_one))
  (bind _defaultsceneroot_2 (Variables|/Game/Blueprints/Doors/Portal.Portal_C|GetDefaultSceneRoot _as_portal_two))
  (bind _transformcomponent (Variables|/Script/Engine.PlayerCameraManager|GetTransformComponent _returnvalue))
  (bind _returnvalue_2 (Transformation|GetWorldRotation _defaultsceneroot))
  (bind _returnvalue_3 (Transformation|GetWorldRotation _defaultsceneroot_2))
  (bind _returnvalue_4 (- (.yaw _returnvalue_2) 1.8e+02))
  (bind _returnvalue_5 (Math|Rotator|MakeRotator (.roll _returnvalue_2) (.pitch _returnvalue_2) _returnvalue_4))
  (bind _returnvalue_6 (Math|Rotator|Delta(Rotator) _returnvalue_5 _returnvalue_3))
  (Transformation|SetWorldLocationAndRotation (Variables|/Game/Blueprints/Doors/Portal.Portal_C|GetCapture (Variables|Default|GetAs%20Portal%20One)) (+ (- (Transformation|GetWorldLocation _defaultsceneroot) (Math|Vector|RotateVector (Transformation|GetWorldLocation _defaultsceneroot_2) _returnvalue_6)) (Math|Vector|RotateVector (Transformation|GetWorldLocation _transformcomponent) _returnvalue_6)) (Math|Rotator|CombineRotators (Transformation|GetWorldRotation _transformcomponent) _returnvalue_6) false false))