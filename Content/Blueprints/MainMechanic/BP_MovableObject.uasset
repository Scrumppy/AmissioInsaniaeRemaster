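; Movable physics object with custom, redirectable gravity that can be grabbed and respawned at its starting location.
; CustomTickPhysics and ResetGravity are mutually exclusive 0.01-second delay loops that add a velocity each step, each clamped to its own max speed.
; BeginPlay starts downward gravity from the player character's DefaultGravity; while grabbed, the loops add nothing.
; Respawn restores a hardcoded downward gravity and moves the mesh back to its saved location.
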(event Custom|CustomTickPhysics
  (params (Target%20Velocity :type Vector))
  (bind _returnvalue (Transformation|GetVelocity))
  (Variables|Default|SetIsResetGravityActive false)
  (Variables|Default|SetIsCustomTickActive true)
  (Variables|Default|SetVelocity Target%20Velocity)
  (if (Variables|Default|GetIsCustomTickActive) :!label _label
    (Utilities|FlowControl|RetriggerableDelay 0.01)
    (Utilities|FlowControl|Sequence
      (:then_0
        (goto _label))
      (:then_1
        (if (Variables|Default|GetBeingGrabbed)
          (Class|PrimitiveComponent|SetAllPhysicsLinearVelocity (Variables|Default|GetObjectMesh) "0, 0, 0" true)
          (elif (not (> (Math|Vector|VectorLengthSquared _returnvalue) (Variables|Default|GetMaxVelocitySquared)))
            (Class|PrimitiveComponent|SetAllPhysicsLinearVelocity (Variables|Default|GetObjectMesh) (Variables|Default|GetVelocity) true)
            (else
              (Class|PrimitiveComponent|SetAllPhysicsLinearVelocity (Variables|Default|GetObjectMesh) (Math|Vector|ClampVectorSize _returnvalue 0.0 (Variables|Default|GetMaxVelocity)) false))))))))

(event Custom|ResetGravity
  (params (Reset%20Velocity :type Vector))
  (bind _returnvalue (Transformation|GetVelocity))
  (Variables|Default|SetIsCustomTickActive false)
  (Variables|Default|SetIsResetGravityActive true)
  (Variables|Default|SetResetVelocity Reset%20Velocity)
  (if (Variables|Default|GetIsResetGravityActive) :!label _label
    (Utilities|FlowControl|RetriggerableDelay 0.01)
    (Utilities|FlowControl|Sequence
      (:then_0
        (goto _label))
      (:then_1
        (if (Variables|Default|GetBeingGrabbed)
          (Class|PrimitiveComponent|SetAllPhysicsLinearVelocity (Variables|Default|GetObjectMesh) "0, 0, 0" true)
          (elif (not (> (Math|Vector|VectorLengthSquared _returnvalue) (Variables|Default|GetMaxVelocitySquaredResetGravity)))
            (Class|PrimitiveComponent|SetAllPhysicsLinearVelocity (Variables|Default|GetObjectMesh) (Variables|Default|GetResetVelocity) true)
            (else
              (Class|PrimitiveComponent|SetAllPhysicsLinearVelocity (Variables|Default|GetObjectMesh) (Math|Vector|ClampVectorSize _returnvalue 0.0 (Variables|Default|GetMaxVelocityResetGravity)) false))))))))

(event EventBeginPlay
  (Variables|Default|SetRespawnLocation (Transformation|GetWorldLocation (Variables|Default|GetObjectMesh)))
  (bind _asfirst_person_character (Utilities|Casting|CastToFirstPersonCharacter (Game|GetPlayerCharacter 0)))
  (bind _output_get (Variables|Default|SetCharacterReference _asfirst_person_character))
  (bind _output_get_2 (Variables|Default|SetVelocity (Math|Vector|MakeVector 0.0 0.0 (* (Variables|/Game/Blueprints/Player/FirstPersonCharacter.FirstPersonCharacter_C|GetDefaultGravity _output_get) -1.0))))
  (CallFunction|ResetGravity _output_get_2)
  (Variables|Default|SetMaxVelocitySquared (Math|Float|Square (Variables|Default|GetMaxVelocity)))
  (Variables|Default|SetMaxVelocitySquaredResetGravity (Math|Float|Square (Variables|Default|GetMaxVelocityResetGravity))))

(fn ConstructionScript)

(fn Respawn
  (bind _returnvalue (* 19.6 -1.0))
  (Class|PrimitiveComponent|SetAllPhysicsLinearVelocity (Variables|Default|GetObjectMesh) (Math|Vector|MakeVector 0.0 0.0 _returnvalue) false)
  (CallFunction|ResetGravity (Math|Vector|MakeVector 0.0 0.0 _returnvalue))
  (Transformation|SetWorldLocation (Variables|Default|GetObjectMesh) (Variables|Default|GetRespawnLocation) false false))