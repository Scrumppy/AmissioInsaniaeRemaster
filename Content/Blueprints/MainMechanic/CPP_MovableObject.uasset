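; Movable physics object with a set mass that applies its own gravity, taken from the player character's default gravity.
; BeginPlay passes that downward vector to CustomTickPhysics, which loops on a 0.01-second retriggerable delay instead of Tick.
; Each step adds the vector to the mesh's linear velocity, or clamps speed once it exceeds MaxVelocity.
; While grabbed, the object receives no added velocity.
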(event Custom|CustomTickPhysics
  (params (Target%20Velocity :type Vector))
  (bind _returnvalue (Transformation|GetVelocity))
  (Variables|Default|SetVelocity Target%20Velocity)
  (if true :!label _label
    (Utilities|FlowControl|RetriggerableDelay 0.01)
    (Utilities|FlowControl|Sequence
      (:then_0
        (goto _label))
      (:then_1
        (if (Utilities|Enum|Equal(Enum) (Variables|/Script/Engine.SceneComponent|GetMobility (Variables|Default|GetObjectMesh)) "Movable")
          (if (Variables|Default|GetBeingGrabbed)
            (Class|PrimitiveComponent|SetAllPhysicsLinearVelocity (Variables|Default|GetObjectMesh) "0, 0, 0" true)
            (elif (not (> (Math|Vector|VectorLengthSquared _returnvalue) (Variables|Default|GetMaxVelocitySquared)))
              (Class|PrimitiveComponent|SetAllPhysicsLinearVelocity (Variables|Default|GetObjectMesh) (Variables|Default|GetVelocity) true)
              (else
                (Class|PrimitiveComponent|SetAllPhysicsLinearVelocity (Variables|Default|GetObjectMesh) (Math|Vector|ClampVectorSize _returnvalue 0.0 (Variables|Default|GetMaxVelocity)) false)))))))))

(event EventBeginPlay
  (Class|PrimitiveComponent|SetMassOverrideinKg (Variables|Default|GetObjectMesh) "None" (Variables|Default|GetMass%20in%20Kg) true)
  (bind _asfirst_person_character (Utilities|Casting|CastToFirstPersonCharacter (Game|GetPlayerCharacter 0)))
  (bind _output_get (Variables|Default|SetCharacterReference _asfirst_person_character))
  (bind _output_get_2 (Variables|Default|SetVelocity (Math|Vector|MakeVector 0.0 0.0 (* (Variables|/Game/Blueprints/Player/FirstPersonCharacter.FirstPersonCharacter_C|GetDefaultGravity _output_get) -1.0))))
  (CallFunction|CustomTickPhysics _output_get_2)
  (Variables|Default|SetMaxVelocitySquared (Math|Float|Square (Variables|Default|GetMaxVelocity))))

(fn ConstructionScript)