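; Actor Blueprint in the main-mechanic folder that traces and draws the direction of its GravityDirection component.
; BeginPlay starts CustomTickPhysics, an endless self-looping event that uses a short retriggerable delay as a custom tick.
; Each pass fires a debug-drawn Visibility line trace along the component's forward vector.
; The trace result and TargetVelocity input are unused, and no dot product is computed despite the name.
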(event Custom|CustomTickPhysics
  (params (Target%20Velocity :type Vector))
  (bind _gravitydirection (Variables|Default|GetGravityDirection))
  (bind _returnvalue (Transformation|GetWorldLocation _gravitydirection))
  (if true :!label _label
    (Utilities|FlowControl|RetriggerableDelay 0.01)
    (Utilities|FlowControl|Sequence
      (:then_0
        (goto _label))
      (:then_1
        (Collision|LineTraceByChannel _returnvalue (+ _returnvalue (* (Math|Vector|GetForwardVector _gravitydirection) 3e+02)) "TraceTypeQuery1" false 0 "ForDuration" true "(R=1.000000,G=0.000000,B=0.000000,A=1.000000)" "(R=0.000000,G=1.000000,B=0.000000,A=1.000000)" 0.2)))))

(event EventBeginPlay
  (CallFunction|CustomTickPhysics (stale Custom|CustomTickPhysics Target%20Velocity)))

(event Collision|EventActorBeginOverlap
  (params (OtherActor :type Actor%20Object%20Reference)))

(event EventTick
  (params (DeltaSeconds :type Float%20%28single-precision%29)))

(fn ConstructionScript)