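; BP_ForceField is a sliding gate in the PressurePlates set that also sends movable objects back to respawn.
; ActivateField eases GateMesh over one second to the ArrivalScenePoint location when open, or back to the relative location cached at BeginPlay when closed.
; Any BP_MovableObject that begins overlapping CollisionBox has Respawn called on it after a short delay, with no check on the open state.
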(event OnComponentBeginOverlap(CollisionBox)
  (params (OverlappedComponent :type Primitive%20Component%20Object%20Reference) (OtherActor :type Actor%20Object%20Reference) (OtherComp :type Primitive%20Component%20Object%20Reference) (OtherBodyIndex :type Integer) (bFromSweep :type Boolean) (SweepResult :type Hit%20Result%20Structure%20%28by%20ref%29))
  (bind _asbp_movable_object (Utilities|Casting|CastToBP_MovableObject OtherActor))
  (Utilities|IsValid _asbp_movable_object
    (:Is%20Valid
      (Utilities|FlowControl|Delay 0.1)
      (Default|Respawn _asbp_movable_object))))

(event Custom|ActivateField
  (params (Is%20Open? :type Boolean))
  (bind _arrivalscenepoint (Variables|Default|GetArrivalScenePoint))
  (bind _default_relative_location (Variables|Default|GetDefault%20Relative%20Location))
  (bind _relativelocation (Variables|/Script/Engine.SceneComponent|GetRelativeLocation _arrivalscenepoint))
  (bind _output_get (Variables|Default|SetIsOpen Is%20Open?))
  (if _output_get
    (Components|MoveComponentTo (Variables|Default|GetGateMesh) (Math|Vector|MakeVector (.x _relativelocation) (.y _relativelocation) (.z _relativelocation)) "0, 0, 0" true true 1.0 false)
    (else
      (Components|MoveComponentTo (Variables|Default|GetGateMesh) (Math|Vector|MakeVector (.x _default_relative_location) (.y _default_relative_location) (.z _default_relative_location)) "0, 0, 0" true true 1.0 false))))

(event EventBeginPlay
  (Variables|Default|SetDefault%20Relative%20Location (Variables|/Script/Engine.SceneComponent|GetRelativeLocation (Variables|Default|GetGateMesh))))

(fn ConstructionScript)