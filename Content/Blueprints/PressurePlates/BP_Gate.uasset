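; Gate actor, in a pressure plate folder, whose mesh slides between a closed and an open position.
; BeginPlay caches the mesh's starting relative location as the closed position.
; ActivateGate takes an IsOpen flag and uses an eased MoveComponentTo to move the mesh to the ArrivalScenePoint component's relative location, or back to the cached start.
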(event Custom|ActivateGate
  (params (Is%20Open? :type Boolean))
  (bind _arrivalscenepoint (Variables|Default|GetArrivalScenePoint))
  (bind _default_relative_location (Variables|Default|GetDefault%20Relative%20Location))
  (bind _relativelocation (Variables|/Script/Engine.SceneComponent|GetRelativeLocation _arrivalscenepoint))
  (bind _output_get (Variables|Default|SetIsOpen Is%20Open?))
  (if _output_get
    (Components|MoveComponentTo (Variables|Default|GetGateMesh) (Math|Vector|MakeVector (.x _relativelocation) (.y _relativelocation) (.z _relativelocation)) "0, 0, 0" true true 1.0 false)
    (else
      (Components|MoveComponentTo (Variables|Default|GetGateMesh) (Math|Vector|MakeVector (.x _default_relative_location) (.y _default_relative_location) (.z _default_relative_location)) "0, 0, 0" true true 1.0 false))))

(event EventBeginPlay
  (Variables|Default|SetDefault%20Relative%20Location (Variables|/Script/Engine.SceneComponent|GetRelativeLocation (Variables|Default|GetGateMesh))))

(fn ConstructionScript)