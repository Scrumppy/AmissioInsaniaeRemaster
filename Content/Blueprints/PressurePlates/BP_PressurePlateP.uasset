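; Pressure plate actor that activates a linked Gate while something overlaps its PressureTrigger and deactivates it when an overlap ends.
; Each overlap event, if the Gate is valid, calls ActivateGate and eases the plate mesh over one second to ArrivalScenePoint or back to DefaultRelativeLocation.
; Overlaps are neither filtered nor counted.
; Older MoveGate logic and the capture of DefaultRelativeLocation sit disconnected, so that default is never set in these graphs.
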(event OnComponentEndOverlap(PressureTrigger)
  (params (OverlappedComponent :type Primitive%20Component%20Object%20Reference) (OtherActor :type Actor%20Object%20Reference) (OtherComp :type Primitive%20Component%20Object%20Reference) (OtherBodyIndex :type Integer))
  (bind _gate (Variables|LinkedGate|GetGate))
  (bind _default_relative_location (Variables|Default|GetDefault%20Relative%20Location))
  (Utilities|IsValid _gate
    (:Is%20Valid
      (Default|ActivateGate _gate false)
      (Components|MoveComponentTo (Variables|Default|GetPressurePlateMesh) (Math|Vector|MakeVector (.x _default_relative_location) (.y _default_relative_location) (.z _default_relative_location)) "0, 0, 0" true true 1.0 false))))

(event OnComponentBeginOverlap(PressureTrigger)
  (params (OverlappedComponent :type Primitive%20Component%20Object%20Reference) (OtherActor :type Actor%20Object%20Reference) (OtherComp :type Primitive%20Component%20Object%20Reference) (OtherBodyIndex :type Integer) (bFromSweep :type Boolean) (SweepResult :type Hit%20Result%20Structure%20%28by%20ref%29))
  (bind _arrivalscenepoint (Variables|Default|GetArrivalScenePoint))
  (bind _gate (Variables|LinkedGate|GetGate))
  (bind _relativelocation (Variables|/Script/Engine.SceneComponent|GetRelativeLocation _arrivalscenepoint))
  (Utilities|IsValid _gate
    (:Is%20Valid
      (Default|ActivateGate _gate true)
      (Components|MoveComponentTo (Variables|Default|GetPressurePlateMesh) (Math|Vector|MakeVector (.x _relativelocation) (.y _relativelocation) (.z _relativelocation)) "0, 0, 0" true true 1.0 false))))

(event EventBeginPlay)

(fn ConstructionScript)